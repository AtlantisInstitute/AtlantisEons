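; Component that gives its owning Character a dash ability with altered movement and visual effects.
; StartDash saves and overrides movement settings, spawns a Dash_BP actor that also receives Jump calls, sets mesh visibility and attaches burst, body and socket-based anim trail particles.
; EndDash destroys that actor, restores saved movement, collision and visibility, and stops the effects.
; Tick then optionally interpolates the mesh back to its default relative location and rotation.
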(event EventBeginPlay
  ;[0.4452 0.6332 1] Store the owner of this component as a character.
  (bind _ascharacter (Utilities|Casting|CastToCharacter (Components|GetOwner)))
  (Variables|Private|Setcharacter _ascharacter)
  ;[0.5979 0.889 1] If the character mesh has not been manually set, find the default one.
  (Utilities|IsValid (Variables|FXSettings|GetCharacterMesh)
    (:Is%20Not%20Valid
      (Variables|FXSettings|SetCharacterMesh (Variables|/Script/Engine.Character|GetMesh (Variables|Private|Getcharacter))))))

(event EventTick
  (params (DeltaSeconds :type Float%20%28single-precision%29))
  (bind _charactermesh (Variables|FXSettings|GetCharacterMesh))
  (bind _charactermesh_2 (Variables|FXSettings|GetCharacterMesh))
  (Variables|Private|SetdeltaTime DeltaSeconds)
  (Utilities|IsValid (Variables|Private|Getcharacter)
    (:Is%20Valid
      (if (Variables|FXSettings|GetshouldMoveCharacterMesh)
        ;[0.8881 1 0.6159] Adjust the character mesh relative location and rotation back to their defaults
        (Utilities|FlowControl|Sequence
          (:then_0
            (if (Variables|Private|Getrotating)
              (Transformation|SetRelativeRotation _charactermesh (Math|Interpolation|RInterpTo (Variables|/Script/Engine.SceneComponent|GetRelativeRotation _charactermesh) (Variables|FXSettings|GetmeshDefaultRelativeRotation) (Variables|Private|GetdeltaTime) (Variables|FXSettings|GetrotationSpeed)) false false)
              (if (Math|Rotator|Equal(Rotator) (Math|Interpolation|RInterpTo (Variables|/Script/Engine.SceneComponent|GetRelativeRotation _charactermesh) (Variables|FXSettings|GetmeshDefaultRelativeRotation) (Variables|Private|GetdeltaTime) (Variables|FXSettings|GetrotationSpeed)) (Variables|FXSettings|GetmeshDefaultRelativeRotation) 1.0)
                (Variables|Private|Setrotating false))))
          (:then_1
            (if (Variables|Private|Getmoving)
              (Transformation|SetRelativeLocation _charactermesh_2 (Math|Interpolation|VInterpTo (Variables|/Script/Engine.SceneComponent|GetRelativeLocation _charactermesh_2) (Variables|FXSettings|GetmeshGroundOffset) (Variables|Private|GetdeltaTime) (Variables|FXSettings|GetmoveSpeed)) false false)
              (if (Math|Vector|Equal(Vector) (Math|Interpolation|VInterpTo (Variables|/Script/Engine.SceneComponent|GetRelativeLocation _charactermesh_2) (Variables|FXSettings|GetmeshGroundOffset) (Variables|Private|GetdeltaTime) (Variables|FXSettings|GetmoveSpeed)) (Variables|FXSettings|GetmeshGroundOffset) 1.0)
                (Variables|Private|Setmoving false)))))))))

(fn StartDash
  (bind _character (Variables|Private|Getcharacter))
  (bind _charactermesh (Variables|FXSettings|GetCharacterMesh))
  (bind _charactermovement (Variables|/Script/Engine.Character|GetCharacterMovement _character))
  (Utilities|IsValid _character
    (:Is%20Valid
      ;[1 0.8741 0.6372] Keep track of the character movement settings before dashing.
      (Variables|Private|SetoldWalkSpeed (Variables|/Script/Engine.CharacterMovementComponent|GetMaxWalkSpeed _charactermovement))
      (Variables|/Script/Engine.CharacterMovementComponent|SetMaxWalkSpeed _charactermovement (Variables|MoveSettings|GetdashWalkSpeed))
      (Variables|Private|SetoldFlySpeed (Variables|/Script/Engine.CharacterMovementComponent|GetMaxFlySpeed _charactermovement))
      (Variables|/Script/Engine.CharacterMovementComponent|SetMaxFlySpeed _charactermovement (Variables|MoveSettings|GetdashFlySpeed))
      (Variables|Private|SetoldAirControl (Variables|/Script/Engine.CharacterMovementComponent|GetAirControl _charactermovement))
      (Variables|/Script/Engine.CharacterMovementComponent|SetAirControl _charactermovement (Variables|MoveSettings|GetdashAirControl))
      (Variables|Private|SetoldAcceleration (Class|CharacterMovementComponent|GetMaxAcceleration _charactermovement))
      (Variables|/Script/Engine.CharacterMovementComponent|SetMaxAcceleration _charactermovement (Variables|MoveSettings|GetdashAcceleration))
      (Variables|Private|SetoldJumpVelocity (Variables|/Script/Engine.CharacterMovementComponent|GetJumpZVelocity _charactermovement))
      (Variables|/Script/Engine.CharacterMovementComponent|SetJumpZVelocity _charactermovement (Variables|MoveSettings|GetdashJumpVelocity))
      (Variables|Private|SetoldMovementMode (Variables|/Script/Engine.CharacterMovementComponent|GetMovementMode _charactermovement))
      (bind _returnvalue (Game|SpawnActorfromClass "/Game/Dash/Dash/Blueprints/Dash_BP.Dash_BP_C" (Math|Transform|MakeTransform "0, 0, 0" "0, 0, 0" "1.000000,1.000000,1.000000") "Undefined" "OverrideRootScale" 0 self 0))
      (Variables|Private|SetdashBP _returnvalue)
      (Private|StartDashTrails)
      (Variables|Private|SetoldMeshVisibility (Variables|/Script/Engine.SceneComponent|GetbVisible _charactermesh))
      (Rendering|SetVisibility _charactermesh (Variables|FXSettings|GetdashMeshVisibility) false)
      (Variables|Private|SetoldCapsuleCollision (Collision|GetCollisionEnabled (Variables|/Script/Engine.Character|GetCapsuleComponent (Variables|Private|Getcharacter))))
      (Variables|Private|SetisDashing true))))

(fn EndDash
  (bind _dashbp (Variables|Private|GetdashBP))
  (bind _character (Variables|Private|Getcharacter))
  (bind _charactermovement (Variables|/Script/Engine.Character|GetCharacterMovement _character))
  (if (Variables|Private|GetisDashing)
    (Variables|Private|SetisDashing false)
    (Utilities|IsValid _dashbp
      (:Is%20Valid
        (Actor|DestroyActor _dashbp)
        ;[0.4452 1 0.6332] Reset character movement settings back to what they were before dashing.
        (Pawn|Components|CharacterMovement|SetMovementMode (Variables|/Script/Engine.Character|GetCharacterMovement (Variables|Private|Getcharacter)) (Variables|Private|GetoldMovementMode) 0)
        (Collision|SetCollisionEnabled (Variables|/Script/Engine.Character|GetCapsuleComponent (Variables|Private|Getcharacter)) (Variables|Private|GetoldCapsuleCollision))
        (Variables|/Script/Engine.CharacterMovementComponent|SetMaxWalkSpeed _charactermovement (Variables|Private|GetoldWalkSpeed))
        (Variables|/Script/Engine.CharacterMovementComponent|SetMaxFlySpeed _charactermovement (Variables|Private|GetoldFlySpeed))
        (Variables|/Script/Engine.CharacterMovementComponent|SetAirControl _charactermovement (Variables|Private|GetoldAirControl))
        (Variables|/Script/Engine.CharacterMovementComponent|SetMaxAcceleration _charactermovement (Variables|Private|GetoldAcceleration))
        (Variables|/Script/Engine.CharacterMovementComponent|SetJumpZVelocity _charactermovement (Variables|Private|GetoldJumpVelocity))
        (Variables|Private|Setrotating true)
        (Variables|Private|Setmoving true)
        (Rendering|SetVisibility (Variables|/Script/Engine.Character|GetMesh (Variables|Private|Getcharacter)) (Variables|Private|GetoldMeshVisibility) false)
        (Private|EndDashTrails)))))

(fn StartDashTrails
  (bind _dashbodyparticles (Variables|FXSettings|GetdashBodyParticles))
  (bind _dashanimtrailparticles (Variables|FXSettings|GetdashAnimTrailParticles))
  (bind _bodyburstparticles (Variables|FXSettings|GetbodyBurstParticles))
  ;[1 0.9982 0.2532] Spawn burst of particles at beginning of dash.
  (Utilities|IsValid _bodyburstparticles
    (:Is%20Valid
      (bind _returnvalue (Effects|SpawnEmitterAttached _bodyburstparticles (Variables|FXSettings|GetCharacterMesh) "None"))
      (Effects|Components|ParticleSystem|SetActorParameter _returnvalue "VertSurfaceActor" (Variables|Private|Getcharacter))
      (Utilities|IsValid _dashbodyparticles
        (:Is%20Valid
          ;[1 0.6462 0.3571] Spawn the particles that will stream off the mesh while dashing.
          (bind _returnvalue_2 (Effects|SpawnEmitterAttached _dashbodyparticles (Variables|FXSettings|GetCharacterMesh) "None"))
          (bind _output_get (Variables|Private|SetbodyParticles _returnvalue_2))
          (Effects|Components|ParticleSystem|SetActorParameter _output_get "VertSurfaceActor" (Variables|Private|Getcharacter))
          ;[1 0.473 0.6349] Spawn the anim trail particles.
          (for (_array_element _array_index) (Variables|FXSettings|GettrailFirstSockets)
            (Utilities|IsValid _dashanimtrailparticles
              (:Is%20Valid
                (bind _returnvalue_3 (Effects|SpawnEmitterAttached _dashanimtrailparticles (Variables|FXSettings|GetCharacterMesh) "None"))
                (Utilities|Array|Add (Variables|Private|Gettrails) _returnvalue_3)
                (Effects|Particles|Trails|BeginTrails _returnvalue_3 _array_element (Utilities|Array|Get(acopy) (Variables|FXSettings|GettrailSecondSockets) _array_index) "ETrailWidthMode_FromCentre" (Variables|FXSettings|GetstreakTrailWidth))))))))))

(fn EndDashTrails
  (bind _bodyparticles (Variables|Private|GetbodyParticles))
  ;[0.8655 0.3674 1] Destroy all the dash fx particles.
  (Utilities|IsValid (Variables|FXSettings|GetbodyBurstParticles)
    (:Is%20Valid
      (Utilities|IsValid _bodyparticles
        (:Is%20Valid
          (Components|Activation|Deactivate _bodyparticles)
          (for _array_element (Variables|Private|Gettrails)
            (Utilities|IsValid _array_element
              (:Is%20Valid
                (Effects|Particles|Trails|EndTrails _array_element)))))))))

(fn Jump
  (Default|Jump (Variables|Private|GetdashBP)))