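; Dash actor that drives a DashComponent's character forward, knocking back and damaging characters it rams, or climbing walls it meets.
; Each tick a forward trace picks between running, hitting or climbing; a capsule hit event also catches rammed characters.
; Climbing uses flying mode without capsule collision, launching upward until an upward trace finds a ceiling, while the mesh interpolates onto the surface.
; Jump kicks off walls, briefly blocking re-climbing.
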(event Custom|Jump
  (bind _dashcomponent (Variables|Private|GetdashComponent))
  (bind _currentnormal (Variables|Private|GetcurrentNormal))
  (bind _dashjumpvelocity (Variables|/Game/Dash/Dash/Blueprints/Dash_Component.Dash_Component_C|GetdashJumpVelocity _dashcomponent))
  (bind _returnvalue (* _currentnormal _dashjumpvelocity))
  (if (Variables|Private|Getwalling)
    ;[1 0.6498 0.4034] Launch the character away from the wall to jump while wall climbing.
    (Character|LaunchCharacter (Variables|/Game/Dash/Dash/Blueprints/Dash_Component.Dash_Component_C|Getcharacter _dashcomponent) (Math|Vector|MakeVector (.x _returnvalue) (.y _returnvalue) _dashjumpvelocity) true true)
    (Variables|Private|SetcanWall false)
    (Utilities|FlowControl|Delay (Variables|/Game/Dash/Dash/Blueprints/Dash_Component.Dash_Component_C|GetjumpWallResetTime (Variables|Private|GetdashComponent)))
    (Variables|Private|SetcanWall true)
    (else
      (Character|Jump (Variables|/Game/Dash/Dash/Blueprints/Dash_Component.Dash_Component_C|Getcharacter (Variables|Private|GetdashComponent))))))

(event Custom|hitCapsuleEvent
  (params (HitComponent :type Primitive%20Component%20Object%20Reference) (OtherActor :type Actor%20Object%20Reference) (OtherComp :type Primitive%20Component%20Object%20Reference) (NormalImpulse :type Vector) (Hit :type Hit%20Result%20Structure%20%28by%20ref%29))
  (bind _dashcomponent (Variables|Private|GetdashComponent))
  (bind _dashcomponent_2 (Variables|Private|GetdashComponent))
  (bind _dashcomponent_3 (Variables|Private|GetdashComponent))
  (bind _dashlaunchstrength (Variables|/Game/Dash/Dash/Blueprints/Dash_Component.Dash_Component_C|GetdashLaunchStrength _dashcomponent_2))
  (bind _character (Variables|/Game/Dash/Dash/Blueprints/Dash_Component.Dash_Component_C|Getcharacter _dashcomponent_3))
  (bind _returnvalue (Pawn|GetControlRotation _character :!class /Script/Engine.Pawn))
  (bind _returnvalue_2 (Math|Vector|GetForwardVector _returnvalue))
  (bind _returnvalue_3 (* _returnvalue_2 _dashlaunchstrength))
  ;[0.9826 1 0.3848] Set up event to push another character when the owning characters capsule hits a character while dashing.
  (if (and (Variables|/Game/Dash/Dash/Blueprints/Dash_Component.Dash_Component_C|GetisDashing _dashcomponent) (Variables|/Game/Dash/Dash/Blueprints/Dash_Component.Dash_Component_C|GetcanDashHitCharacter _dashcomponent))
    (Utilities|IsValid OtherActor
      (:Is%20Valid
        (bind _ascharacter (Utilities|Casting|CastToCharacter OtherActor))
        (Class|DashInterface|HitCharacter(Message) (Variables|/Game/Dash/Dash/Blueprints/Dash_Component.Dash_Component_C|Getcharacter (Variables|Private|GetdashComponent)) _ascharacter)
        (Default|EndDash (Variables|Private|GetdashComponent))
        (Character|LaunchCharacter _ascharacter (Math|Vector|MakeVector (.x _returnvalue_3) (.y _returnvalue_3) 0.0) false false)
        (Game|Damage|ApplyDamage _ascharacter (Variables|/Game/Dash/Dash/Blueprints/Dash_Component.Dash_Component_C|GetcharacterHitDamage (Variables|Private|GetdashComponent)) (Pawn|GetController _character) _character (Variables|/Game/Dash/Dash/Blueprints/Dash_Component.Dash_Component_C|GetcharacterHitDamageType (Variables|Private|GetdashComponent)))))))

(event EventBeginPlay
  ;[0.9826 1 0.3848] Set up event to push another character when the owning characters capsule hits a character while dashing.
  (Collision|BindEventtoOnComponentHit (Variables|/Script/Engine.Character|GetCapsuleComponent (Variables|/Game/Dash/Dash/Blueprints/Dash_Component.Dash_Component_C|Getcharacter (Variables|Private|GetdashComponent))) (delegate Custom|hitCapsuleEvent)))

(event EventTick
  (params (DeltaSeconds :type Float%20%28single-precision%29))
  (Variables|Private|SetdeltaSec DeltaSeconds)
  (CallFunction|TraceForward)
  (CallFunction|MoveMesh))

(fn ConstructionScript)

(fn MoveMesh
  (bind _dashcomponent (Variables|Private|GetdashComponent))
  (bind _charactermesh (Variables|/Game/Dash/Dash/Blueprints/Dash_Component.Dash_Component_C|GetCharacterMesh _dashcomponent))
  ;[0.3528 0.3871 1] Change the relative location and rotation of the owning characters mesh.
  (if (Variables|/Game/Dash/Dash/Blueprints/Dash_Component.Dash_Component_C|GetshouldMoveCharacterMesh _dashcomponent)
    (Transformation|SetWorldLocationAndRotation _charactermesh (Math|Interpolation|VInterpTo (Transformation|GetWorldLocation _charactermesh) (Variables|Private|GettargetMeshLoc) (Variables|Private|GetdeltaSec) (Variables|/Game/Dash/Dash/Blueprints/Dash_Component.Dash_Component_C|GetmoveSpeed (Variables|Private|GetdashComponent))) (Math|Interpolation|RInterpTo (Transformation|GetWorldRotation _charactermesh) (Variables|Private|GettargetMeshRot) (Variables|Private|GetdeltaSec) (Variables|/Game/Dash/Dash/Blueprints/Dash_Component.Dash_Component_C|GetrotationSpeed (Variables|Private|GetdashComponent))) false false)))

(fn TraceForward
  (bind _dashcomponent (Variables|Private|GetdashComponent))
  (bind _dashcomponent_2 (Variables|Private|GetdashComponent))
  (bind _dashcomponent_3 (Variables|Private|GetdashComponent))
  (bind _character (Variables|/Game/Dash/Dash/Blueprints/Dash_Component.Dash_Component_C|Getcharacter _dashcomponent_3))
  (bind _character_2 (Variables|/Game/Dash/Dash/Blueprints/Dash_Component.Dash_Component_C|Getcharacter _dashcomponent))
  (bind _returnvalue (Transformation|GetActorLocation _character_2))
  ;[1 0.3638 0.7846] Trace forward from the character.
  (bind _outhit (Collision|LineTraceByChannel _returnvalue (+ _returnvalue (* (Transformation|GetActorForwardVector _character_2) (Variables|/Game/Dash/Dash/Blueprints/Dash_Component.Dash_Component_C|GettraceDistance _dashcomponent_2))) (Variables|/Game/Dash/Dash/Blueprints/Dash_Component.Dash_Component_C|GetdashTraceChannel _dashcomponent_2) false (Utilities|Array|MakeArray _character_2) "None"))
  (if (.bBlockingHit (Collision|BreakHitResult _outhit))
    ;[0.3265 0.5582 1] If something is hit, store hit variables, and check to see if characters can be hit or not.
    (Variables|Private|SettargetMeshLoc (+ (.ImpactPoint (Collision|BreakHitResult _outhit)) (* (.Normal (Collision|BreakHitResult _outhit)) (Variables|/Game/Dash/Dash/Blueprints/Dash_Component.Dash_Component_C|GetmeshWallOffset (Variables|Private|GetdashComponent)))))
    (Variables|Private|SetcurrentNormal (.Normal (Collision|BreakHitResult _outhit)))
    (Variables|Private|SetcurActor (.HitActor (Collision|BreakHitResult _outhit)))
    (if (Variables|/Game/Dash/Dash/Blueprints/Dash_Component.Dash_Component_C|GetcanDashHitCharacter (Variables|Private|GetdashComponent))
      (CallFunction|LaunchCharacter)
      (else
        (CallFunction|MoveActor)))
    (else
      ;[0.3851 1 0.8899] If nothing is hit, move forward.
      (Pawn|Input|AddMovementInput _character (Math|Vector|GetForwardVector (Pawn|GetControlRotation _character :!class /Script/Engine.Pawn)) 1.0 false)
      (CallFunction|LeaveWall))))

(fn LaunchCharacter
  (bind _dashcomponent (Variables|Private|GetdashComponent))
  (bind _curactor (Variables|Private|GetcurActor))
  (bind _dashcomponent_2 (Variables|Private|GetdashComponent))
  (bind _dashcomponent_3 (Variables|Private|GetdashComponent))
  (bind _dashlaunchstrength (Variables|/Game/Dash/Dash/Blueprints/Dash_Component.Dash_Component_C|GetdashLaunchStrength _dashcomponent_3))
  (bind _character (Variables|/Game/Dash/Dash/Blueprints/Dash_Component.Dash_Component_C|Getcharacter _dashcomponent))
  (bind _character_2 (Variables|/Game/Dash/Dash/Blueprints/Dash_Component.Dash_Component_C|Getcharacter _dashcomponent_2))
  (bind _returnvalue (Pawn|GetControlRotation _character :!class /Script/Engine.Pawn))
  (bind _returnvalue_2 (Math|Vector|GetForwardVector _returnvalue))
  (bind _returnvalue_3 (* _returnvalue_2 _dashlaunchstrength))
  (Utilities|IsValid _curactor
    (:Is%20Valid
      ;[1 0.09697 0.01729] If a character has been hit, stop dashing, launch the character, and apply damage to them.
      (bind _ascharacter (Utilities|Casting|CastToCharacter _curactor)
        (:then
          (Variables|Private|SetcurCharacter _ascharacter)
          (Default|EndDash (Variables|Private|GetdashComponent))
          (Class|DashInterface|HitCharacter(Message) _character (Variables|Private|GetcurCharacter))
          (Character|LaunchCharacter (Variables|Private|GetcurCharacter) (Math|Vector|MakeVector (.x _returnvalue_3) (.y _returnvalue_3) _dashlaunchstrength) true true)
          (Game|Damage|ApplyDamage (Variables|Private|GetcurCharacter) (Variables|/Game/Dash/Dash/Blueprints/Dash_Component.Dash_Component_C|GetcharacterHitDamage _dashcomponent_2) (Pawn|GetController _character_2) _character_2 (Variables|/Game/Dash/Dash/Blueprints/Dash_Component.Dash_Component_C|GetcharacterHitDamageType _dashcomponent_2)))
        (:CastFailed
          (CallFunction|MoveActor :!label _label))))
    (:Is%20Not%20Valid
      (goto _label))))

(fn MoveActor
  (bind _dashcomponent (Variables|Private|GetdashComponent))
  (bind _dashcomponent_2 (Variables|Private|GetdashComponent))
  (bind _dashcomponent_3 (Variables|Private|GetdashComponent))
  (bind _dashjumpvelocity (Variables|/Game/Dash/Dash/Blueprints/Dash_Component.Dash_Component_C|GetdashJumpVelocity _dashcomponent))
  (bind _character (Variables|/Game/Dash/Dash/Blueprints/Dash_Component.Dash_Component_C|Getcharacter _dashcomponent_2))
  (bind _character_2 (Variables|/Game/Dash/Dash/Blueprints/Dash_Component.Dash_Component_C|Getcharacter _dashcomponent_3))
  (bind _returnvalue (Transformation|GetActorRotation _character_2))
  (bind _returnvalue_2 (Math|Rotator|MakeRotator 0.0 0.0 (.yaw _returnvalue)))
  (bind _returnvalue_3 (Math|Vector|GetForwardVector _returnvalue_2))
  (bind _returnvalue_4 (* _returnvalue_3 _dashjumpvelocity))
  (if (and (Variables|Private|GetcanWall) (Variables|/Game/Dash/Dash/Blueprints/Dash_Component.Dash_Component_C|GetcanDashOnWall (Variables|Private|GetdashComponent)))
    ;[0.4958 1 0.1912] Start climbing a wall.
    (Variables|Private|SettargetMeshRot (Math|Rotator|MakeRotfromZ (Variables|Private|GetcurrentNormal)))
    (Variables|Private|Setwalling true)
    (Pawn|Components|CharacterMovement|SetMovementMode (Variables|/Script/Engine.Character|GetCharacterMovement _character) "MOVE_Flying" 0)
    (Collision|SetCollisionEnabled (Variables|/Script/Engine.Character|GetCapsuleComponent _character) "NoCollision")
    (CallFunction|TraceUp)
    (else
      ;[0.1009 1 0.5975] Stop climbing a wall.
      (Variables|Private|SettargetCharLoc (+ (Transformation|GetActorLocation (Variables|/Game/Dash/Dash/Blueprints/Dash_Component.Dash_Component_C|Getcharacter (Variables|Private|GetdashComponent))) (Math|Vector|MakeVector (.x _returnvalue_4) (.y _returnvalue_4) 0.0)))
      (CallFunction|LeaveWall))))

(fn LeaveWall
  (bind _dashcomponent (Variables|Private|GetdashComponent))
  (bind _character (Variables|/Game/Dash/Dash/Blueprints/Dash_Component.Dash_Component_C|Getcharacter _dashcomponent))
  (bind _capsulecomponent (Variables|/Script/Engine.Character|GetCapsuleComponent _character))
  ;[0 1 0.9459] Reset relative mesh location and rotation, and turn capsule collision back on.
  (Variables|Private|SettargetMeshRot (Math|Rotator|CombineRotators (Variables|/Game/Dash/Dash/Blueprints/Dash_Component.Dash_Component_C|GetmeshDefaultRelativeRotation _dashcomponent) (Math|Rotator|MakeRotator 0.0 0.0 (.yaw (Pawn|GetControlRotation _character :!class /Script/Engine.Pawn)))))
  (Variables|Private|SettargetMeshLoc (+ (Transformation|GetWorldLocation _capsulecomponent) (Variables|/Game/Dash/Dash/Blueprints/Dash_Component.Dash_Component_C|GetmeshGroundOffset (Variables|Private|GetdashComponent))))
  (Variables|Private|Setwalling false)
  (Collision|SetCollisionEnabled _capsulecomponent "QueryAndPhysics"))

(fn TraceUp
  (bind _dashcomponent (Variables|Private|GetdashComponent))
  (bind _dashcomponent_2 (Variables|Private|GetdashComponent))
  (bind _charactermesh (Variables|/Game/Dash/Dash/Blueprints/Dash_Component.Dash_Component_C|GetCharacterMesh _dashcomponent_2))
  (bind _tracedistance (Variables|/Game/Dash/Dash/Blueprints/Dash_Component.Dash_Component_C|GettraceDistance _dashcomponent))
  (bind _returnvalue (Transformation|GetWorldLocation _charactermesh))
  (bind _returnvalue_2 (Math|Vector|GetUpVector _charactermesh))
  (bind _returnvalue_3 (* _returnvalue_2 _tracedistance))
  (bind _returnvalue_4 (+ _returnvalue _returnvalue_3))
  ;[0.2436 0.141 1] Trace up from character to check for ceiling. If there is none, keep moving up.
  (bind _outhit (Collision|LineTraceByChannel _returnvalue_4 (+ _returnvalue_4 (Variables|/Game/Dash/Dash/Blueprints/Dash_Component.Dash_Component_C|GettraceUpHeightOffset _dashcomponent)) "TraceTypeQuery1" false (Utilities|Array|MakeArray (Variables|/Game/Dash/Dash/Blueprints/Dash_Component.Dash_Component_C|Getcharacter _dashcomponent)) "None"))
  (if (.bBlockingHit (Collision|BreakHitResult _outhit))
    (Variables|/Script/Engine.MovementComponent|SetVelocity (Variables|/Script/Engine.Character|GetCharacterMovement (Variables|/Game/Dash/Dash/Blueprints/Dash_Component.Dash_Component_C|Getcharacter (Variables|Private|GetdashComponent))) "0, 0, 0")
    (else
      (Character|LaunchCharacter (Variables|/Game/Dash/Dash/Blueprints/Dash_Component.Dash_Component_C|Getcharacter (Variables|Private|GetdashComponent)) (* (Math|Vector|GetUpVector (Math|Conversions|RotationFromXVector (Variables|Private|GetcurrentNormal))) (Variables|/Game/Dash/Dash/Blueprints/Dash_Component.Dash_Component_C|GetwallMoveSpeed (Variables|Private|GetdashComponent))) true true))))