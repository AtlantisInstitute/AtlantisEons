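; Basic projectile actor for the Shield FX Responsive asset, handling what happens when its sphere hits something.
; On hit, it deactivates its Niagara effect, then hides the sphere and turns off its physics and collision.
; A second sequence branch spawns the hit Niagara system at the impact location using the actor's rotation.
; Both branches end in a delayed destroy, so the shorter delay on the effect branch removes the actor.
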(event OnComponentHit(Sphere)
  (params (HitComponent :type Primitive%20Component%20Object%20Reference) (OtherActor :type Actor%20Object%20Reference) (OtherComp :type Primitive%20Component%20Object%20Reference) (NormalImpulse :type Vector :default "0, 0, 0") (Hit :type Hit%20Result%20Structure%20%28by%20ref%29))
  (bind _sphere (Variables|Default|GetSphere))
  (Utilities|FlowControl|Sequence
    (:then_0
      (Components|Activation|Deactivate (Variables|Default|GetNiagara))
      (Physics|SetSimulatePhysics _sphere false)
      (Collision|SetCollisionEnabled _sphere "NoCollision")
      (Rendering|SetVisibility _sphere false false)
      (Utilities|FlowControl|Delay 4.0)
      (Actor|DestroyActor))
    (:then_1
      (Niagara|SpawnSystematLocation "/Game/Shield_FX_Responsive/forUe5_2version/Niagara/Projectile/NS_Projectile_Hit.NS_Projectile_Hit" (.Location (Collision|BreakHitResult Hit)) (Transformation|GetActorRotation))
      (Utilities|FlowControl|Delay 3.0)
      (Actor|DestroyActor))))

(fn ConstructionScript)