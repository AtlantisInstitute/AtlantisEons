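; BP_Shooting_Small is a shooter actor that continuously spawns small projectiles of the ProjectileBP class from BeginPlay onward.
; NextArrow spawns each one at reduced scale, aimed along the Arrow component, then re-calls itself after a short random delay.
; Spawn points are randomly offset from the actor, with the ShootongHeight range driving both X and Z and a fixed range spreading Y.
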(event Custom|NextArrow
  (bind _shootong_height_min (Variables|Default|GetShootong%20height%20Min))
  (bind _shootong_height_max (Variables|Default|GetShootong%20height%20Max))
  (bind _returnvalue (Math|Random|RandomFloatinRange _shootong_height_min _shootong_height_max))
  (Game|SpawnActorfromClass (Variables|Default|GetProjectileBP) (Math|Transform|MakeTransform (+ (Transformation|GetActorLocation) (Math|Vector|MakeVector _returnvalue (Math|Random|RandomFloatinRange -5e+01 1.5e+03) _returnvalue)) (.rotation (Transformation|GetWorldTransform (Variables|Default|GetArrow))) "0.100000,0.100000,0.100000") "Undefined" "SelectDefaultAtRuntime" 0 0)
  (Utilities|FlowControl|Delay (Math|Random|RandomFloatinRange 0.0 0.1))
  (CallFunction|NextArrow))

(event EventBeginPlay
  (bind _shootong_height_min (Variables|Default|GetShootong%20height%20Min))
  (bind _shootong_height_max (Variables|Default|GetShootong%20height%20Max))
  (bind _returnvalue (Math|Random|RandomFloatinRange _shootong_height_min _shootong_height_max))
  (Utilities|FlowControl|Delay (Math|Random|RandomFloatinRange 0.0 0.1))
  (Game|SpawnActorfromClass (Variables|Default|GetProjectileBP) (Math|Transform|MakeTransform (+ (Transformation|GetActorLocation) (Math|Vector|MakeVector _returnvalue (Math|Random|RandomFloatinRange -5e+01 1.5e+03) _returnvalue)) (.rotation (Transformation|GetWorldTransform (Variables|Default|GetArrow))) "0.100000,0.100000,0.100000") "Undefined" "SelectDefaultAtRuntime" 0 0)
  (Utilities|FlowControl|Delay (Math|Random|RandomFloatinRange 0.0 0.1))
  (CallFunction|NextArrow))

(fn ConstructionScript)