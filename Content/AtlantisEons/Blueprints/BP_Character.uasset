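; Player character Blueprint that adds a blink dash and prepares circular HP and MP bar materials.
; Dodge input or touch press picks a forward or backward dash, then brackets the blinkDashFX effect with DashComponent start and end calls.
; The effect receives a Niagara shadow system, camera FOV and movement references, and is updated on Tick.
; The construction script creates both dynamic bar materials from M_Circular and initializes them.
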(event Input|EnhancedActionEvents|EnhancedInputActionIA_Dodge
  (params (ActionValue :type Vector%202D%20Structure) (ElapsedSeconds :type Float%20%28double-precision%29) (TriggeredSeconds :type Float%20%28double-precision%29) (InputAction :type Input%20Action%20Object%20Reference :default "/Game/AtlantisEons/Input/Actions/IA_Dodge.IA_Dodge"))
  (bind _returnvalue (Class|AtlantisEonsCharacter|ShouldDashForward))
  (bind _dash_component (Variables|Default|GetDash_Component))
  ;[0.15 0.15 0.15 0.5] Dash Component
  (:Started
    (if _returnvalue
      (Variables|Default|SetDash%20Distance 1e+03)
      (else
        (Variables|Default|SetDash%20Distance -1e+03)))
    (Default|StartDash _dash_component)
    (Utilities|BlinkDashFX (Variables|Character|GetCharacterMovement) (Variables|Default|GetDash%20Distance) "/Game/BlinkAndDashVFX/VFX_Niagara/NS_Dash_Shadow.NS_Dash_Shadow" 0 self (Variables|Default|GetCapsuleComponent) 0.4 (stale EventTick DeltaSeconds) (Variables|Default|GetFollowCamera) false true 0.1 9e+01 _returnvalue
      (:Out
        (Default|EndDash _dash_component)))))

(event EventTick
  (params (DeltaSeconds :type Float%20%28single-precision%29))
  ;[0.15 0.15 0.15 0.5] Dash Component
  (Utilities|BlinkDashFX (Variables|Character|GetCharacterMovement) (Variables|Default|GetDash%20Distance) "/Game/BlinkAndDashVFX/VFX_Niagara/NS_Dash_Shadow.NS_Dash_Shadow" 0 self (Variables|Default|GetCapsuleComponent) 0.4 DeltaSeconds (Variables|Default|GetFollowCamera) false true 0.1 9e+01 (Class|AtlantisEonsCharacter|ShouldDashForward)) ; enters at EventTick
)

(event EventOnTouchDashPressed
  (bind _returnvalue (Class|AtlantisEonsCharacter|ShouldDashForward))
  (bind _dash_component (Variables|Default|GetDash_Component))
  ;[0.15 0.15 0.15 0.5] Dash Component
  (if _returnvalue
    (Variables|Default|SetDash%20Distance 1e+03)
    (else
      (Variables|Default|SetDash%20Distance -1e+03)))
  (Default|StartDash _dash_component)
  (Utilities|BlinkDashFX (Variables|Character|GetCharacterMovement) (Variables|Default|GetDash%20Distance) "/Game/BlinkAndDashVFX/VFX_Niagara/NS_Dash_Shadow.NS_Dash_Shadow" 0 self (Variables|Default|GetCapsuleComponent) 0.4 (stale EventTick DeltaSeconds) (Variables|Default|GetFollowCamera) false true 0.1 9e+01 _returnvalue
    (:Out
      (Default|EndDash _dash_component))))

(fn ConstructionScript
  ;[1 1 1] Creating Dynamic Material for Circular Bar and Initail Setting
  (bind _returnvalue (Rendering|Material|CreateDynamicMaterialInstance "/Game/AtlantisEons/Materials/M_Circular.M_Circular" "" "None" :!class /Script/Engine.KismetMaterialLibrary))
  (Variables|Default|SetCircularHP _returnvalue)
  (bind _returnvalue_2 (Rendering|Material|CreateDynamicMaterialInstance "/Game/AtlantisEons/Materials/M_Circular.M_Circular" "" "None" :!class /Script/Engine.KismetMaterialLibrary))
  (Variables|Default|SetCircularMP _returnvalue_2)
  (Class|AtlantisEonsCharacter|SettingCircularBarHP)
  (Class|AtlantisEonsCharacter|SettingCircularBarMP))