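; BP_Item is a ground item actor, either placed or spawned when the player drops an item with an index and stack count.
; It reads Table_ItemList, async-loads the mesh, orients it by equip slot, and creates a name widget showing stack counts for unequippable items.
; Tick projects the widget to screen space.
; Sphere overlaps with the character's "ItemBoundary"-tagged component toggle the widget and update the character's BPItemRef list.
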(event OnComponentBeginOverlap(Sphere)
  (params (OverlappedComponent :type Primitive%20Component%20Object%20Reference) (OtherActor :type Actor%20Object%20Reference) (OtherComp :type Primitive%20Component%20Object%20Reference) (OtherBodyIndex :type Integer) (bFromSweep :type Boolean) (SweepResult :type Hit%20Result%20Structure%20%28by%20ref%29))
  (bind _itemnameref (Variables|Default|GetItemNameRef))
  ;[1 1 1] Set Item Name Widget interaction which is pop-up event when you come close to an Item actor.
  (bind _asbp_character (Utilities|Casting|CastToBP_Character OtherActor))
  (if (Components|ComponentHasTag OtherComp "ItemBoundary")
    (Utilities|IsValid _itemnameref
      (:Is%20Valid
        (Default|StopAnimation _itemnameref)
        (UserInterface|Viewport|AddtoViewport _itemnameref 0)
        (Default|ItemNameShow _itemnameref)
        (Utilities|Array|Add (Variables|/Game/AtlantisEons/Blueprints/BP_Character.BP_Character_C|GetBPItemRef _asbp_character) self)))))

(event OnComponentEndOverlap(Sphere)
  (params (OverlappedComponent :type Primitive%20Component%20Object%20Reference) (OtherActor :type Actor%20Object%20Reference) (OtherComp :type Primitive%20Component%20Object%20Reference) (OtherBodyIndex :type Integer))
  (bind _itemnameref (Variables|Default|GetItemNameRef))
  ;[1 1 1] Set Item Name Widget interaction which is pop-up event when you come close to an Item actor.
  (bind _asbp_character (Utilities|Casting|CastToBP_Character OtherActor))
  (if (Components|ComponentHasTag OtherComp "ItemBoundary")
    (Utilities|IsValid _itemnameref
      (:Is%20Valid
        (Widget|RemovefromParent _itemnameref)
        (Default|ItemNameHide _itemnameref)
        (Utilities|Array|RemoveItem (Variables|/Game/AtlantisEons/Blueprints/BP_Character.BP_Character_C|GetBPItemRef _asbp_character) self)))))

(event Custom|SpawnItem
  (params (ItemIndex :type Integer) (StackNumber :type Integer))
  (bind _staticmesh (Variables|Default|GetStaticMesh))
  ;[1 1 1] Spawning an item when you throw away the item on the ground with information of item index and stack number.
  (Variables|Default|SetItemIndex ItemIndex)
  (Variables|Default|SetStackNumber StackNumber)
  (bind _asbp_character (Utilities|Casting|CastToBP_Character (Game|GetPlayerCharacter 0)))
  (Utilities|Array|Add (Variables|/Game/AtlantisEons/Blueprints/BP_Character.BP_Character_C|GetBPItemRef _asbp_character) self)
  ;[1 1 1] Spawning an item when creating this blueprint class.
  (bind _returnvalue (Utilities|GetDataTableRow "/Game/AtlantisEons/Blueprints/InventoryandEquipment/Table_ItemList.Table_ItemList" (Utilities|String|StringToName (Utilities|String|ToString(Integer) (Variables|Default|GetItemIndex))))
    (:then
      (Variables|Default|SetItemTable _returnvalue)
      (bind _object (Utilities|AsyncLoadAsset (.Item3DModel (Utilities|Struct|BreakStructure_ItemInfo _returnvalue)))
        (:Completed
          (bind _asstatic_mesh (Utilities|Casting|CastToStaticMesh _object))
          (Components|StaticMesh|SetStaticMesh (Variables|Default|GetStaticMesh) _asstatic_mesh)
          ;[1 1 1] Create Item Name Widget
          (bind _returnvalue_2 (UserInterface|CreateWidget "/Game/AtlantisEons/Blueprints/InventoryandEquipment/WBP_ItemNamePopUp.WBP_ItemNamePopUp_C" (Game|GetPlayerController 0)))
          (Variables|Default|SetItemNameRef _returnvalue_2)
          ;[1 1 1] Rotate item axis and change Y scale of a spawning item on the ground depending on an item form factor.
          (switch Utilities|FlowControl|Switch|SwitchonEnum_ItemEquipSlot (.ItemEquipSlot (Utilities|Struct|BreakStructure_ItemInfo _returnvalue))
            (:NewEnumerator0
              ;[1 1 1] Set item name and stack number information.
              (Variables|/Game/AtlantisEons/Blueprints/InventoryandEquipment/WBP_ItemNamePopUp.WBP_ItemNamePopUp_C|SetItemName (Variables|Default|GetItemNameRef) (.ItemName (Utilities|Struct|BreakStructure_ItemInfo (Variables|Default|GetItemTable))) :!label _label))
            (:NewEnumerator1
              (Transformation|SetRelativeRotation _staticmesh "90.000000,0.000000,-90.000000" false false)
              (goto _label))
            (:NewEnumerator9
              (Transformation|SetRelativeScale3D _staticmesh "1.000000,0.400000,1.000000")
              (Transformation|SetRelativeRotation _staticmesh "0.000000,0.000000,-90.000000" false false)
              (goto _label))
            (:NewEnumerator2
              (Transformation|SetRelativeRotation _staticmesh "0.000000,0.000000,-90.000000" false false)
              (goto _label))
            (:NewEnumerator8
              (Transformation|SetRelativeRotation _staticmesh "0, 0, 0" false false)
              (if (> (Variables|Default|GetStackNumber) 1)
                (Variables|/Game/AtlantisEons/Blueprints/InventoryandEquipment/WBP_ItemNamePopUp.WBP_ItemNamePopUp_C|SetItemName (Variables|Default|GetItemNameRef) (Utilities|String|Append (.ItemName (Utilities|Struct|BreakStructure_ItemInfo (Variables|Default|GetItemTable))) " 
" "[" (Utilities|String|ToString(Integer) (Variables|Default|GetStackNumber)) "]"))
                (else
                  (goto _label)))))
          (Class|UserWidget|SetAlignmentinViewport (Variables|Default|GetItemNameRef) "(X=0.500000,Y=1.000000)"))))))

(event Custom|RemoveItemNameWidget
  (bind _itemnameref (Variables|Default|GetItemNameRef))
  ;[1 1 1] When Opening UMG, remove item name widgets
  (Utilities|IsValid _itemnameref
    (:Is%20Valid
      (Widget|RemovefromParent _itemnameref))))

(event EventBeginPlay
  (bind _stacknumber (Variables|Default|GetStackNumber))
  (bind _staticmesh (Variables|Default|GetStaticMesh))
  ;[1 1 1] Spawning an item when creating this blueprint class.
  (bind _returnvalue (Utilities|GetDataTableRow "/Game/AtlantisEons/Blueprints/InventoryandEquipment/Table_ItemList.Table_ItemList" (Utilities|String|StringToName (Utilities|String|ToString(Integer) (Variables|Default|GetItemIndex))))
    (:then
      (Variables|Default|SetItemTable _returnvalue)
      (bind _object (Utilities|AsyncLoadAsset (.Item3DModel (Utilities|Struct|BreakStructure_ItemInfo _returnvalue)))
        (:Completed
          (bind _asstatic_mesh (Utilities|Casting|CastToStaticMesh _object))
          (Components|StaticMesh|SetStaticMesh (Variables|Default|GetStaticMesh) _asstatic_mesh)
          ;[1 1 1] Create Item Name Widget
          (bind _returnvalue_2 (UserInterface|CreateWidget "/Game/AtlantisEons/Blueprints/InventoryandEquipment/WBP_ItemNamePopUp.WBP_ItemNamePopUp_C" (Game|GetPlayerController 0)))
          (Variables|Default|SetItemNameRef _returnvalue_2)
          ;[1 1 1] Rotate item axis and change Y scale of a spawning item on the ground depending on an item form factor.
          (switch Utilities|FlowControl|Switch|SwitchonEnum_ItemEquipSlot (.ItemEquipSlot (Utilities|Struct|BreakStructure_ItemInfo _returnvalue))
            (:NewEnumerator0
              ;[1 1 1] Set item name and stack number information.
              (Variables|/Game/AtlantisEons/Blueprints/InventoryandEquipment/WBP_ItemNamePopUp.WBP_ItemNamePopUp_C|SetItemName (Variables|Default|GetItemNameRef) (.ItemName (Utilities|Struct|BreakStructure_ItemInfo (Variables|Default|GetItemTable))) :!label _label))
            (:NewEnumerator1
              (Transformation|SetRelativeRotation _staticmesh "90.000000,0.000000,-90.000000" false false)
              (goto _label))
            (:NewEnumerator9
              (Transformation|SetRelativeScale3D _staticmesh "1.000000,0.400000,1.000000")
              (Transformation|SetRelativeRotation _staticmesh "0.000000,0.000000,-90.000000" false false)
              (goto _label))
            (:NewEnumerator2
              (Transformation|SetRelativeRotation _staticmesh "0.000000,0.000000,-90.000000" false false)
              (goto _label))
            (:NewEnumerator8
              (Transformation|SetRelativeRotation _staticmesh "0, 0, 0" false false)
              (if (> _stacknumber 1)
                (Variables|/Game/AtlantisEons/Blueprints/InventoryandEquipment/WBP_ItemNamePopUp.WBP_ItemNamePopUp_C|SetItemName (Variables|Default|GetItemNameRef) (Utilities|String|Append (.ItemName (Utilities|Struct|BreakStructure_ItemInfo (Variables|Default|GetItemTable))) " 
" "[" (Utilities|String|ToString(Integer) _stacknumber) "]"))
                (else
                  (goto _label)))))
          (Class|UserWidget|SetAlignmentinViewport (Variables|Default|GetItemNameRef) "(X=0.500000,Y=1.000000)"))))))

(event EventTick
  (params (DeltaSeconds :type Float%20%28single-precision%29))
  (bind _returnvalue (Game|GetPlayerController 0))
  (bind _returnvalue_2 (Transformation|GetActorLocation))
  (bind _itemnameref (Variables|Default|GetItemNameRef))
  (bind (_screenlocation _returnvalue_3) (Class|PlayerController|ProjectWorldLocationtoScreen _returnvalue _returnvalue_2 false))
  ;[1 1 1] Set Item Name Widget Position to screen
  (Utilities|IsValid (Variables|Default|GetItemNameRef)
    (:Is%20Valid
      (if _returnvalue_3
        (Widget|SetVisibility _itemnameref "Visible")
        (Class|UserWidget|SetPositioninViewport _itemnameref _screenlocation true)
        (else
          (Widget|SetVisibility _itemnameref "Collapsed"))))))

(fn ConstructionScript)